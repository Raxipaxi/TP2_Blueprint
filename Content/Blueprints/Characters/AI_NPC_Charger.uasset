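; AI_NPC_Charger is a charger NPC character that reacts to perceived stimuli and respawns the player on contact.
; Perception updates write the stimulus location and sensed state to the HearingLocation and IsHearing blackboard keys.
; A Box overlap with BP_Player calls its FadeOutRespawn.
; BeginPlay applies MaxSpeed as walk speed, and UpdateStimuli requests a perception listener update.
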(event OnComponentBeginOverlap(Box)
  (params (OverlappedComponent :type Primitive%20Component%20Object%20Reference) (OtherActor :type Actor%20Object%20Reference) (OtherComp :type Primitive%20Component%20Object%20Reference) (OtherBodyIndex :type Integer) (bFromSweep :type Boolean) (SweepResult :type Hit%20Result%20Structure%20%28by%20ref%29))
  (bind _asbp_player (Utilities|Casting|CastToBP_Player OtherActor))
  (Default|FadeOutRespawn _asbp_player))

(event OnTargetPerceptionUpdated(AIPerception)
  (params (Actor :type Actor%20Object%20Reference) (Stimulus :type AI%20Stimulus%20Structure))
  (bind (_age _expirationage _strength _stimuluslocation _receiverlocation _tag _bsuccessfullysensed) (Utilities|Struct|BreakAIStimulus Stimulus))
  (bind _returnvalue (AI|GetBlackboard 0))
  ;[1 1 1] Si percibe algo guarda su posicion y actualiza el bool de percepcion en el blackboard
  (AI|Components|Blackboard|SetValueasVector _returnvalue (Utilities|Name|MakeLiteralName "HearingLocation") _stimuluslocation)
  (AI|Components|Blackboard|SetValueasBool _returnvalue (Utilities|Name|MakeLiteralName "IsHearing") _bsuccessfullysensed))

(event EventBeginPlay
  ;[1 1 1] Para cambiar la velocidad del npc desde editor
  (Variables|/Script/Engine.CharacterMovementComponent|SetMaxWalkSpeed (Variables|Character|GetCharacterMovement) (Variables|Default|GetMaxSpeed)))

(fn ConstructionScript)

(fn UpdateStimuli
  (Class|AIPerceptionComponent|RequestStimuliListenerUpdate (Variables|Default|GetAIPerception)))