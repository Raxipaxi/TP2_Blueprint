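; AI_NPC_Boss is a boss NPC character that damages the player on contact.
; On begin play it sets its walk speed from an editable MaxSpeed variable.
; Capsule overlaps with BP_Player apply Damage through a DoOnce that resets after a two-second delay, acting as a hit cooldown.
; An UpdateStimuli function asks the AI Perception component to refresh its stimuli listener.
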(event OnComponentBeginOverlap(Capsule)
  (params (OverlappedComponent :type Primitive%20Component%20Object%20Reference) (OtherActor :type Actor%20Object%20Reference) (OtherComp :type Primitive%20Component%20Object%20Reference) (OtherBodyIndex :type Integer) (bFromSweep :type Boolean) (SweepResult :type Hit%20Result%20Structure%20%28by%20ref%29))
  (bind _asbp_player (Utilities|Casting|CastToBP_Player OtherActor))
  (Utilities|FlowControl|DoOnce false :!label _label
    (:Completed
      (Game|Damage|ApplyDamage _asbp_player (Variables|Default|GetDamage) 0 0)
      (Utilities|FlowControl|Delay 2.0)
      (goto _label Reset))))

(event EventBeginPlay
  ;[1 1 1] Para cambiar la velocidad del npc desde editor
  (Variables|/Script/Engine.CharacterMovementComponent|SetMaxWalkSpeed (Variables|Character|GetCharacterMovement) (Variables|Default|GetMaxSpeed)))

(fn ConstructionScript)

(fn UpdateStimuli
  (Class|AIPerceptionComponent|RequestStimuliListenerUpdate (Variables|Default|GetAIPerception)))