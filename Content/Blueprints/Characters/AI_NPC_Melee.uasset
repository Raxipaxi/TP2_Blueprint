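; Melee enemy NPC (goblin, per the tutorial kill counter) that damages the player on contact and takes its walk speed from MaxSpeed.
; Sphere overlaps apply damage through a DoOnce that resets after a short cooldown.
; Any nonzero damage ragdolls it, then after a delay reports the kill to the tutorial or level 1 game mode and destroys it.
; Health is unused and DecreaseHealth is empty.
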(event OnComponentBeginOverlap(Sphere)
  (params (OverlappedComponent :type Primitive%20Component%20Object%20Reference) (OtherActor :type Actor%20Object%20Reference) (OtherComp :type Primitive%20Component%20Object%20Reference) (OtherBodyIndex :type Integer) (bFromSweep :type Boolean) (SweepResult :type Hit%20Result%20Structure%20%28by%20ref%29))
  (Utilities|FlowControl|DoOnce false :!label _label
    (:Completed
      (Game|Damage|ApplyDamage (.AsBP%20Player (Utilities|Casting|CastToBP_Player OtherActor)) (Variables|Default|GetDamage) 0 0)
      (Utilities|FlowControl|Delay 1.5)
      (goto _label Reset))))

(event EventBeginPlay
  ;[1 1 1] Para cambiar la velocidad del npc desde editor
  (Variables|/Script/Engine.CharacterMovementComponent|SetMaxWalkSpeed (Variables|Character|GetCharacterMovement) (Variables|Default|GetMaxSpeed))
  (bind _asgm_tuto (Utilities|Casting|CastToGM_Tuto (Game|GetGameMode)))
  (Variables|Default|SetGameMode _asgm_tuto))

(event Game|Damage|EventAnyDamage
  (params (Damage :type Float%20%28single-precision%29) (DamageType :type Damage%20Type%20Object%20Reference) (InstigatedBy :type Controller%20Object%20Reference) (DamageCauser :type Actor%20Object%20Reference))
  (bind _returnvalue (Game|GetGameMode))
  ;[1 1 1] Die
  (if (not (== 0.0 Damage))
    (Physics|SetSimulatePhysics (Variables|Character|GetMesh) true)
    (Utilities|FlowControl|Delay 5.0)
    (bind _asgm_tuto (Utilities|Casting|CastToGM_Tuto _returnvalue)
      (:then
        (Default|GoblinsKills _asgm_tuto))
      (:CastFailed
        (bind _asgm_lvl_1 (Utilities|Casting|CastToGM_Lvl1 _returnvalue)
          (:then
            (Default|CountEnemy _asgm_lvl_1))
          (:CastFailed
            _))))
    (Actor|DestroyActor)))

(fn ConstructionScript)

(fn DecreaseHealth
  (params (Damage :type Float%20%28single-precision%29)))