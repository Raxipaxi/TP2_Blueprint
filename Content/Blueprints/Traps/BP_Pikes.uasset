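; BP_Pikes is a looping spike trap that raises spears and damages actors that touch it.
; On BeginPlay, a timeline lerps the spear mesh upward along Z from its base position, then waits a cooldown and replays.
; A sound plays at the actor location each time the cycle starts.
; Box overlap applies damage on begin overlap, independent of the spears' current position in the cycle.
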(event OnComponentBeginOverlap(Box)
  (params (OverlappedComponent :type Primitive%20Component%20Object%20Reference) (OtherActor :type Actor%20Object%20Reference) (OtherComp :type Primitive%20Component%20Object%20Reference) (OtherBodyIndex :type Integer) (bFromSweep :type Boolean) (SweepResult :type Hit%20Result%20Structure%20%28by%20ref%29))
  ;[1 0.04404 0] Give Damage
  (Game|Damage|ApplyDamage OtherActor (Math|Conversions|ToFloat(Integer) (Variables|Default|GetDamage)) 0 0))

(event Custom|Play%20Effect
  (Audio|PlaySoundatLocation "/Game/Sound/SC_SpikeTrap.SC_SpikeTrap" (Transformation|GetActorLocation) "0, 0, 0" 1.0 1.0 0.0 0 0 0))

(event EventBeginPlay
  ;[0 0.1805 1] Trap Movement
  (bind _output_get (Variables|Default|SetBase%20Location (Variables|/Script/Engine.SceneComponent|GetRelativeLocation (Variables|Default|GetSM_Prop_Trap_Spears_01))))
  (CallFunction|PlayEffect)
  (bind _activation_track (Timeline|Trap%20Activate Play)
    (:Update
      (Transformation|SetRelativeLocation (Variables|Default|GetSM_Prop_Trap_Spears_01) (Math|Vector|Lerp(Vector) _output_get (+ _output_get "0, 0,90.000000") _activation_track) false false))
    (:Finished
      ;;[0.0831 0.9801 1] Reset trap
      (Utilities|FlowControl|Delay (Variables|Default|GetCooldown))
      (CallFunction|PlayEffect)
      (Timeline|Trap%20Activate PlayFromStart))))

(fn ConstructionScript)