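; Spinning saw trap that travels along a straight path and damages actors it hits.
; On BeginPlay a timeline lerps the saw between its starting location and that point plus a Movement offset.
; It tries to invert the RotatingMovement roll near either endpoint, though an author comment says this fails.
; Component hits apply fixed damage through a DoOnce that resets after a short delay, giving one cooldown for all actors.
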(event OnComponentHit(SM_Prop_Trap_Saw_01)
  (params (HitComponent :type Primitive%20Component%20Object%20Reference) (OtherActor :type Actor%20Object%20Reference) (OtherComp :type Primitive%20Component%20Object%20Reference) (NormalImpulse :type Vector :default "0, 0, 0") (Hit :type Hit%20Result%20Structure%20%28by%20ref%29))
  (Utilities|FlowControl|DoOnce false :!label _label
    (:Completed
      (Game|Damage|ApplyDamage OtherActor 12.0 0 0)
      (Utilities|FlowControl|Delay 1.5)
      (goto _label Reset))))

(event Custom|Move
  (bind _sm_prop_trap_saw_01 (Variables|Default|GetSM_Prop_Trap_Saw_01))
  (bind _rotatingmovement (Variables|Default|GetRotatingMovement))
  (bind _returnvalue (Transformation|GetWorldLocation _sm_prop_trap_saw_01))
  (bind _newtrack_0 (Timeline|Timeline_0 Play)
    (:Update
      (Transformation|SetWorldLocation _sm_prop_trap_saw_01 (Math|Vector|Lerp(Vector) (Variables|Default|GetpointA) (Variables|Default|GetpointB) _newtrack_0) false false)
      ;[1 1 1] Cambio de sentido de giro (no funca porque no quiere)
      (if (or (Math|Vector|Equal(Vector) (Variables|Default|GetpointA) _returnvalue 0.05) (Math|Vector|Equal(Vector) _returnvalue (Variables|Default|GetpointB) 0.05))
        (Variables|/Script/Engine.RotatingMovementComponent|SetRotationRate _rotatingmovement (Math|Rotator|MakeRotator (* (.roll (Variables|/Script/Engine.RotatingMovementComponent|GetRotationRate _rotatingmovement)) -1.0) 0.0 0.0))))))

(event EventBeginPlay
  (bind _output_get (Variables|Default|SetpointA (Transformation|GetWorldLocation (Variables|Default|GetSM_Prop_Trap_Saw_01))))
  (Variables|Default|SetpointB (+ _output_get (Variables|Default|GetMovement)))
  (CallFunction|Move))

(fn ConstructionScript)