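; BP_PuzzlePlat is a Level 1 puzzle pressure plate that lights up and sinks when the player steps on it.
; Stepping on an already activated plate restores all activated plates, raising them and switching off their material highlight.
; Each press checks every plate; when all are active, it flags GM_Lvl1's puzzle complete and gives the player a key.
; Movement uses Delay loops stepped by DeltaSeconds cached from Tick.
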(event OnComponentBeginOverlap(Box)
  (params (OverlappedComponent :type Primitive%20Component%20Object%20Reference) (OtherActor :type Actor%20Object%20Reference) (OtherComp :type Primitive%20Component%20Object%20Reference) (OtherBodyIndex :type Integer) (bFromSweep :type Boolean) (SweepResult :type Hit%20Result%20Structure%20%28by%20ref%29))
  ;[1 1 1] Overlap Event
  (bind _asgm_lvl_1 (Utilities|Casting|CastToGM_Lvl1 (Game|GetGameMode)))
  (if (not (Variables|/Game/Blueprints/GameModes/Lvl1/GM_Lvl1.GM_Lvl1_C|GetIsPuzzleCompleted _asgm_lvl_1))
    (Utilities|Casting|CastToBP_Player OtherActor)
    (if (Variables|Default|GetActivated)
      (Utilities|FlowControl|Delay 0.5)
      (CallFunction|ChangeColor false)
      (bind _outactors (Actor|GetAllActorsOfClass "BP_PuzzlePlat_C"))
      (for _array_element _outactors
        (bind _asbp_puzzle_plat (Utilities|Casting|CastToBP_PuzzlePlat _array_element))
        (if (Variables|BP_PuzzlePlat_C|GetActivated _asbp_puzzle_plat)
          (CallFunction|Restore _asbp_puzzle_plat)))
      (else
        (Utilities|FlowControl|Delay 0.1)
        (CallFunction|ChangeColor true)
        (CallFunction|Activate)
        (Utilities|FlowControl|Delay 0.5)
        (CallFunction|CheckforCompletition)))))

(event Custom|Restore
  ;[1 0.3955 0.4154] Restart
  (CallFunction|ChangeColor false)
  (Transformation|SetActorLocation (+ (Transformation|GetActorLocation) (Math|Vector|MakeVector 0.0 0.0 (* (Variables|Default|GetDelta%20Seconds) 1e+02))) false false :!label _label)
  (if (>= (.z (Transformation|GetActorLocation)) (Variables|Default|GetStarterHeight))
    (Variables|Default|SetActivated false)
    (else
      (Utilities|FlowControl|Delay (Variables|Default|GetDelta%20Seconds))
      (goto _label))))

(event Custom|CheckForCompletition
  ;[1 1 1] Completition Checker
  (bind _outactors (Actor|GetAllActorsOfClass "BP_PuzzlePlat_C"))
  (bind _array_element (Utilities|Array|ForEachLoopwithBreak _outactors :!label _label)
    (:LoopBody
      (if (Variables|BP_PuzzlePlat_C|GetActivated _array_element)
        (Variables|Default|SetCompleted true)
        (else
          (Variables|Default|SetCompleted false)
          (goto _label Break))))
    (:Completed
      (if (Variables|Default|GetCompleted)
        (Development|PrintString "COMPLETADO")
        (bind _asgm_lvl_1 (Utilities|Casting|CastToGM_Lvl1 (Game|GetGameMode)))
        (Variables|/Game/Blueprints/GameModes/Lvl1/GM_Lvl1.GM_Lvl1_C|SetIsPuzzleCompleted _asgm_lvl_1 true)
        (Default|AddKey (Variables|/Game/Blueprints/GameModes/Lvl1/GM_Lvl1.GM_Lvl1_C|GetCurrentPlayer _asgm_lvl_1))
        (else
          (Development|PrintString "Cnacelado"))))))

(event Custom|Activate
  ;[0.3091 1 0.3049] Activate
  (CallFunction|ChangeColor true)
  (Transformation|SetActorLocation (- (Transformation|GetActorLocation) (Math|Vector|MakeVector 0.0 0.0 (* (Variables|Default|GetDelta%20Seconds) 1e+02))) false false :!label _label)
  (if (<= (.z (Transformation|GetActorLocation)) (- (Variables|Default|GetStarterHeight) (Variables|Default|GetDisplacement)))
    (Variables|Default|SetActivated true)
    (else
      (Utilities|FlowControl|Delay (Variables|Default|GetDelta%20Seconds))
      (goto _label))))

(event Custom|Change%20Color
  (params (Active :type Boolean))
  (bind _platform (Variables|Default|GetPlatform))
  ;[0 0.1493 1] Color Change
  (if Active
    (Rendering|Material|CreateDynamicMaterialInstance _platform 0 "/Game/Dungeon/Materials/Mat_Dungeon_01.Mat_Dungeon_01" "None" :!class /Script/Engine.PrimitiveComponent)
    (Rendering|Material|SetScalarParameterValueonMaterials _platform "IsActive" 1.0)
    (else
      (Rendering|Material|CreateDynamicMaterialInstance _platform 0 "/Game/Dungeon/Materials/Mat_Dungeon_01.Mat_Dungeon_01" "None" :!class /Script/Engine.PrimitiveComponent)
      (Rendering|Material|SetScalarParameterValueonMaterials _platform "IsActive" 0.0))))

(event EventBeginPlay
  ;[1 1 1] BeginPlay
  (Variables|Default|SetStarterHeight (.Z (Math|Vector|BreakVector (Transformation|GetActorLocation)))))

(event EventTick
  (params (DeltaSeconds :type Float%20%28single-precision%29))
  ;[1 1 1] Tick
  (Variables|Default|SetDelta%20Seconds DeltaSeconds))

(fn ConstructionScript)