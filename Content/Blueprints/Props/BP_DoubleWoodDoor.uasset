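; One-shot double wooden door that opens when the player enters its Open trigger holding enough keys.
; Timelines lerp both leaves' relative rotations to swing them open, and back to their BeginPlay rotations on closing.
; Entering the Close trigger afterwards shuts it for good, resets the player's keys and stops the glow on every door instance.
; StartGlowing and StopGlow toggle the IsReady parameter on dynamic door materials.
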(event OnComponentBeginOverlap(Open)
  (params (OverlappedComponent :type Primitive%20Component%20Object%20Reference) (OtherActor :type Actor%20Object%20Reference) (OtherComp :type Primitive%20Component%20Object%20Reference) (OtherBodyIndex :type Integer) (bFromSweep :type Boolean) (SweepResult :type Hit%20Result%20Structure%20%28by%20ref%29))
  ;[1 1 1] Check Keys
  (bind _asbp_player (Utilities|Casting|CastToBP_Player OtherActor))
  (bind _output_get (Variables|Default|SetPlayer _asbp_player))
  (if (>= (Default|GetKeysQuantity _output_get) (Variables|Default|GetKeysRequired))
    (Utilities|FlowControl|DoOnce false
      (:Completed
        (if (not (Variables|Flag|GetWasClosed))
          (CallFunction|OpenDoors)
          (Variables|Flag|SetDoor%20Opened true))))))

(event OnComponentBeginOverlap(Close)
  (params (OverlappedComponent :type Primitive%20Component%20Object%20Reference) (OtherActor :type Actor%20Object%20Reference) (OtherComp :type Primitive%20Component%20Object%20Reference) (OtherBodyIndex :type Integer) (bFromSweep :type Boolean) (SweepResult :type Hit%20Result%20Structure%20%28by%20ref%29))
  ;[1 1 1] Close after opened
  (if (and (Variables|Flag|GetDoor%20Opened) (not (Variables|Flag|GetWasClosed)))
    (CallFunction|CloseDoors)
    (Variables|Flag|SetWasClosed true)
    (Default|ResetKeys (Variables|Default|GetPlayer))
    (bind _outactors (Actor|GetAllActorsOfClass "BP_DoubleWoodDoor_C"))
    (for _array_element _outactors
      (CallFunction|StopGlow _array_element))))

(event Custom|OpenDoors
  ;[1 1 1] Open Doors
  (if (not (Variables|Flag|GetDoor%20Opened))
    (Utilities|FlowControl|Sequence
      (:then_0
        ;[0.7913 0.6308 0.09759] Left Door Open
        (bind _opens (Timeline|LeftDoorTime Play)
          (:Update
            (Transformation|SetRelativeRotation (Variables|Default|GetLeftDoor) (Math|Rotator|Lerp(Rotator) (Variables|/Script/Engine.SceneComponent|GetRelativeRotation (Variables|Default|GetLeftDoor)) "0, 0, 0" _opens) false false))))
      (:then_1
        ;[0.7913 0.6308 0.09759] Right Door Open
        (bind _opens_2 (Timeline|RightDoorTime PlayFromStart)
          (:Update
            (Transformation|SetRelativeRotation (Variables|Default|GetRightDoor) (Math|Rotator|Lerp(Rotator) (Variables|/Script/Engine.SceneComponent|GetRelativeRotation (Variables|Default|GetRightDoor)) "0,180.000000, 0" _opens_2) false false)))))))

(event Custom|Close%20Doors
  ;[1 1 1] Close Doors
  (if (not (Variables|Flag|GetWasClosed))
    (Utilities|FlowControl|DoOnce false
      (:Completed
        (Utilities|FlowControl|Sequence
          (:then_0
            ;[0.7913 0.6308 0.09759] Left Door Close
            (bind _opens (Timeline|Close%20Left%20Time Play)
              (:Update
                (Transformation|SetRelativeRotation (Variables|Default|GetLeftDoor) (Math|Rotator|Lerp(Rotator) (Variables|/Script/Engine.SceneComponent|GetRelativeRotation (Variables|Default|GetLeftDoor)) (Math|Rotator|MakeRotator 0.0 0.0 9e+01) _opens) false false))
              (:Finished
                (Transformation|SetRelativeRotation (Variables|Default|GetLeftDoor) (Variables|Default|GetInitial%20Rotation%20Left) false false))))
          (:then_1
            ;[0.7913 0.6308 0.09759] Right Door close
            (bind _opens_2 (Timeline|Close%20Right%20Time Play)
              (:Update
                (Transformation|SetRelativeRotation (Variables|Default|GetRightDoor) (Math|Rotator|Lerp(Rotator) (Variables|/Script/Engine.SceneComponent|GetRelativeRotation (Variables|Default|GetRightDoor)) "0,90.000000, 0" _opens_2) false false))
              (:Finished
                (Transformation|SetRelativeRotation (Variables|Default|GetRightDoor) (Variables|Default|GetInitial%20Rotation%20Right) false false)))))))))

(event Custom|Stop%20Glow
  (bind _leftdoor (Variables|Default|GetLeftDoor))
  (bind _rightdoor (Variables|Default|GetRightDoor))
  ;[1 1 1] Stop Glow
  (Rendering|Material|CreateDynamicMaterialInstance _leftdoor 0 "/Game/Materials/M_Doors.M_Doors" "None" :!class /Script/Engine.PrimitiveComponent)
  (Rendering|Material|SetScalarParameterValueonMaterials _leftdoor "IsReady" 0.0)
  (Rendering|Material|CreateDynamicMaterialInstance _rightdoor 0 "/Game/Materials/M_Doors.M_Doors" "None" :!class /Script/Engine.PrimitiveComponent)
  (Rendering|Material|SetScalarParameterValueonMaterials _rightdoor "IsReady" 0.0))

(event Custom|Start%20Glowing
  (bind _leftdoor (Variables|Default|GetLeftDoor))
  (bind _rightdoor (Variables|Default|GetRightDoor))
  ;[1 1 1] Start Glow
  (if (not (Variables|Flag|GetWasClosed))
    (Rendering|Material|CreateDynamicMaterialInstance _leftdoor 0 "/Game/Materials/M_Doors.M_Doors" "None" :!class /Script/Engine.PrimitiveComponent)
    (Rendering|Material|SetScalarParameterValueonMaterials _leftdoor "IsReady" 1.0)
    (Rendering|Material|CreateDynamicMaterialInstance _rightdoor 0 "/Game/Materials/M_Doors.M_Doors" "None" :!class /Script/Engine.PrimitiveComponent)
    (Rendering|Material|SetScalarParameterValueonMaterials _rightdoor "IsReady" 1.0)))

(event EventBeginPlay
  ;[1 1 1] Inicitial Rotator (Doors)
  (Variables|Default|SetInitial%20Rotation%20Right (Variables|/Script/Engine.SceneComponent|GetRelativeRotation (Variables|Default|GetRightDoor)))
  (Variables|Default|SetInitial%20Rotation%20Left (Variables|/Script/Engine.SceneComponent|GetRelativeRotation (Variables|Default|GetLeftDoor))))

(fn ConstructionScript)

(fn OpenRightDoor)

(fn OpenLeftDoor)