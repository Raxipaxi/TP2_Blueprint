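; NPC projectile that flies straight ahead and damages the player on impact.
; A ProjectileStats event sets its lifespan, damage and speed, and Tick moves it forward with a swept local offset instead of a movement component.
; On mesh hit, it damages BP_Player once and destroys itself.
; It ignores ranged and boss NPCs and is destroyed by anything else.
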(event OnComponentHit(Mesh)
  (params (HitComponent :type Primitive%20Component%20Object%20Reference) (OtherActor :type Actor%20Object%20Reference) (OtherComp :type Primitive%20Component%20Object%20Reference) (NormalImpulse :type Vector :default "0, 0, 0") (Hit :type Hit%20Result%20Structure%20%28by%20ref%29))
  (bind _asbp_player (Utilities|Casting|CastToBP_Player OtherActor)
    (:then
      (Utilities|FlowControl|DoOnce false
        (:Completed
          (Game|Damage|ApplyDamage _asbp_player (Variables|Default|GetProjectileDamage) 0 0)
          (Actor|DestroyActor))))
    (:CastFailed
      (Utilities|Casting|CastToAI_NPC_Ranged OtherActor
        (:CastFailed
          (Utilities|Casting|CastToAI_NPC_Boss OtherActor
            (:CastFailed
              (Actor|DestroyActor))))))))

(event Custom|ProjectileStats
  (params (Lifespan :type Float%20%28single-precision%29) (Damage :type Float%20%28single-precision%29) (Speed :type Float%20%28single-precision%29))
  ;[1 1 1] Prepara los stats
  (Actor|SetLifeSpan Lifespan)
  (Variables|Default|SetProjectileSpeed Speed)
  (Variables|Default|SetProjectileDamage Damage))

(event EventTick
  (params (DeltaSeconds :type Float%20%28single-precision%29))
  ;[1 1 1] Va para adelante
  (Transformation|AddActorLocalOffset (* (Class|KismetMathLibrary|VectorForward) (* DeltaSeconds (Variables|Default|GetProjectileSpeed))) true false))

(fn ConstructionScript)