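; Enemy spawner actor that spawns a series of melee or ranged AI enemies, with EnemyIndex selecting the type at BeginPlay.
; After a short delay, the chosen event loops on a SpawnRate delay, cycling through SpawnPoints as offsets from the actor's location.
; The loop stops when SpawnCounter minus one equals EnemyAmount, so a counter starting at zero yields one enemy more than EnemyAmount.
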(event Custom|Spawn%20Melee
  (Utilities|FlowControl|Delay 0.2)
  (AI|SpawnAIFromClass (Variables|Default|GetMelee%20Enemy) 0 (+ (.location (Transformation|GetActorTransform)) (Utilities|Array|Get(acopy) (Variables|Default|GetSpawnPoints) (Variables|Default|GetSpawnIndex))) "0, 0, 0" false 0 :!label _label)
  (Variables|Default|SetSpawnCounter (+ (Variables|Default|GetSpawnCounter) 1))
  (if (== (- (Utilities|Array|Length (Variables|Default|GetSpawnPoints)) 1) (Variables|Default|GetSpawnIndex))
    (Variables|Default|SetSpawnIndex 0)
    (else
      (Variables|Default|SetSpawnIndex (+ (Variables|Default|GetSpawnIndex) 1))))
  (if (not (== (- (Variables|Default|GetSpawnCounter) 1) (Variables|Default|GetEnemyAmount)))
    (Utilities|FlowControl|Delay (Variables|Default|GetSpawnRate))
    (goto _label)))

(event Custom|Spawn%20Range
  (Utilities|FlowControl|Delay 0.2)
  (AI|SpawnAIFromClass (Variables|Default|GetRanged%20Enemy) 0 (+ (.location (Transformation|GetActorTransform)) (Utilities|Array|Get(acopy) (Variables|Default|GetSpawnPoints) (Variables|Default|GetSpawnIndex))) "0, 0, 0" false 0 :!label _label)
  (Variables|Default|SetSpawnCounter (+ (Variables|Default|GetSpawnCounter) 1))
  (if (== (- (Utilities|Array|Length (Variables|Default|GetSpawnPoints)) 1) (Variables|Default|GetSpawnIndex))
    (Variables|Default|SetSpawnIndex 0)
    (else
      (Variables|Default|SetSpawnIndex (+ (Variables|Default|GetSpawnIndex) 1))))
  (if (not (== (- (Variables|Default|GetSpawnCounter) 1) (Variables|Default|GetEnemyAmount)))
    (Utilities|FlowControl|Delay (Variables|Default|GetSpawnRate))
    (goto _label)))

(event EventBeginPlay
  (switch int (Variables|Default|GetEnemy%20Index)
    (:0
      (CallFunction|SpawnMelee))
    (:1
      (CallFunction|SpawnRange))))

(fn ConstructionScript)