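; BP_Pillar is a pillar light that turns on when an actor overlaps it, apparently as a checkpoint marker.
; BeginPlay stores the PointLight's initial intensity and sets the light to zero.
; The first overlap by any actor passes a DoOnce and plays the Lit timeline, whose CheckpointLit track lerps the light back to that intensity.
; A SetNewSpawn call exists but is disconnected, so no spawn point is updated here.
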(event EventBeginPlay
  (bind _pointlight (Variables|Default|GetPointLight))
  (Variables|Default|SetInit%20Intensity (Variables|/Script/Engine.LightComponentBase|GetIntensity _pointlight))
  (Rendering|Components|Light|SetIntensity _pointlight 0.0))

(event Collision|EventActorBeginOverlap
  (params (OtherActor :type Actor%20Object%20Reference))
  (Utilities|FlowControl|DoOnce false
    (:Completed
      (bind _checkpoint_lit (Timeline|Lit Play)
        (:Update
          (Rendering|Components|Light|SetIntensity (Variables|Default|GetPointLight) (Math|Float|Lerp 0.0 (Variables|Default|GetInit%20Intensity) _checkpoint_lit)))))))

(fn ConstructionScript)