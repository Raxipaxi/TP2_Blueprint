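; BP_PillarMaze is a maze pillar light that switches on when the player reaches it.
; BeginPlay stores the light's intensity, darkens it and applies the configured color.
; The first player overlap with the box plays a one-shot timeline that fades intensity back to the stored value.
; A separate Checkpoint Effect graph makes delayed Activate calls on the player's shield effect, but nothing here invokes it.
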(event OnComponentBeginOverlap(Box)
  (params (OverlappedComponent :type Primitive%20Component%20Object%20Reference) (OtherActor :type Actor%20Object%20Reference) (OtherComp :type Primitive%20Component%20Object%20Reference) (OtherBodyIndex :type Integer) (bFromSweep :type Boolean) (SweepResult :type Hit%20Result%20Structure%20%28by%20ref%29))
  (Utilities|IsPlayer OtherActor
    (:IsPlayer
      (Utilities|FlowControl|DoOnce false
        (:Completed
          (bind _checkpoint_lit (Timeline|Lit Play)
            (:Update
              (Rendering|Components|Light|SetIntensity (Variables|Default|GetPointLight) (Math|Float|Lerp 0.0 (Variables|Default|GetInit%20Intensity) _checkpoint_lit)))))))))

(event EventBeginPlay
  (bind _pointlight (Variables|Default|GetPointLight))
  (Variables|Default|SetInit%20Intensity (Variables|/Script/Engine.LightComponentBase|GetIntensity _pointlight))
  (Rendering|Components|Light|SetIntensity _pointlight 0.0)
  (Rendering|Components|Light|SetLightColor (Variables|Default|GetPointLight) (Variables|Default|GetColor) true))

(fn ConstructionScript)