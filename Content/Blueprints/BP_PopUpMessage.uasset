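; BP_PopUpMessage is a trigger box actor that shows an on-screen message when BP_Player overlaps it.
; Each player overlap destroys the optional Dependent actor, then passes a DoOnce that blocks repeat messages while one is showing.
; A W_Message widget displays the Message variable for the Lifesawn delay and is then removed.
; The trigger then destroys itself if Destructible, or resets the DoOnce for reuse.
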(event OnComponentBeginOverlap(Box)
  (params (OverlappedComponent :type Primitive%20Component%20Object%20Reference) (OtherActor :type Actor%20Object%20Reference) (OtherComp :type Primitive%20Component%20Object%20Reference) (OtherBodyIndex :type Integer) (bFromSweep :type Boolean) (SweepResult :type Hit%20Result%20Structure%20%28by%20ref%29))
  (Utilities|Casting|CastToBP_Player OtherActor)
  (if (not (== (Variables|Default|GetDependent) 0))
    (Actor|DestroyActor (Variables|Default|GetDependent)))
  (Utilities|FlowControl|DoOnce false :!label _label
    (:Completed
      (bind _returnvalue (UserInterface|CreateWidget "/Game/Blueprints/UI/W_Message.W_Message_C"))
      (Variables|/Game/Blueprints/UI/W_Message.W_Message_C|SetMessage _returnvalue (Variables|Default|GetMessage))
      (UserInterface|Viewport|AddtoViewport _returnvalue 0)
      (Utilities|FlowControl|Delay (Variables|Default|GetLifesawn))
      (Widget|RemovefromParent _returnvalue)
      (if (Variables|Default|GetDestructible)
        (Actor|DestroyActor)
        (else
          (goto _label Reset))))))

(event EventBeginPlay)

(event Collision|EventActorBeginOverlap
  (params (OtherActor :type Actor%20Object%20Reference)))

(event EventTick
  (params (DeltaSeconds :type Float%20%28single-precision%29)))

(fn ConstructionScript)