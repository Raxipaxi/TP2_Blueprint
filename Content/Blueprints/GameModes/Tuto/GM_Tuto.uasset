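; GM_Tuto is the tutorial Game Mode, handling first-section loading, player retries and goblin-kill progress.
; BeginPlay streams in L_TutoSection1 and caches the player pawn and its HUD widget.
; CheckTriesAndDead, not started within this file, re-calls itself on a short delay, spending a try on death and reviving the player unless none remain.
; GoblinsKills counts kills, awarding a key and resetting at ten.
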(event Custom|Check%20Tries%20And%20Dead
  ;[1 1 1] Dead Check
  (if (Default|IsAlive (Variables|Default|GetPlayer))
    _
    (else
      (bind _output_get (Variables|Default|SetTries (- (Variables|Default|GetTries) 1)))
      (if (== _output_get 0)
        _
        (else
          (Default|SetDeadFalse (Variables|Default|GetPlayer))))))
  (Utilities|FlowControl|Delay 0.2)
  (CallFunction|CheckTriesandDead))

(event Custom|GoblinsKills
  ;[1 1 1] Goblins Counter and key achieve
  (bind _output_get (Variables|Default|SetGoblinsCounter (+ (Variables|Default|GetGoblinsCounter) 1)))
  (if (== _output_get 10)
    (Default|PickKey (Variables|Default|GetPlayer))
    (Variables|Default|SetGoblinsCounter 0)))

(event EventBeginPlay
  ;[0.04501 1 0.3754] Load first Stream Level
  (Game|LoadStreamLevel(byName) "L_TutoSection1" true)
  ;[0 0.9418 1] Get player ref
  (bind _asbp_player (Utilities|Casting|CastToBP_Player (Game|Player|GetPlayerPawn 0)))
  (Variables|Default|SetPlayer _asbp_player)
  ;[1 1 1] Get HUD Widget
  (Variables|Default|SetHUD (Variables|/Game/Blueprints/Characters/BP_Player.BP_Player_C|GetAs%20W%20Player%20HUD (Variables|Default|GetPlayer))))

(fn ConstructionScript)